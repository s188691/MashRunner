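; BP_Field is a Paper2D playfield that builds itself to a configurable length in its construction script.
; It tiles StageParts + 1 field sprites along X at StageLength spacing.
; The BoxTop and BotBottom box components are resized and centred to span the row, and GoalTop and GoalBottom shift along X by StageParts times StageLength.
; The event graph holds no runtime logic.
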(fn `UserConstructionScript`
  (bind _boxtop (`self.BoxTop`))
  (bind _boxtop_2 (`self.BoxTop`))
  (bind _botbottom (`self.BotBottom`))
  (bind _goalbottom (`self.GoalBottom`))
  (bind _botbottom_2 (`self.BotBottom`))
  (bind _goaltop (`self.GoalTop`))
  (bind _stageparts (`self.StageParts`))
  (bind (_relativelocation_x _relativelocation_y _relativelocation_z) (`KismetMathLibrary.BreakVector` (`SceneComponent.RelativeLocation` _botbottom_2)))
  (bind (_relativelocation_x_2 _relativelocation_y_2 _relativelocation_z_2) (`KismetMathLibrary.BreakVector` (`SceneComponent.RelativeLocation` _boxtop)))
  (bind (_relativelocation_x_3 _relativelocation_y_3 _relativelocation_z_3) (`KismetMathLibrary.BreakVector` (`SceneComponent.RelativeLocation` _goalbottom)))
  (bind (_relativelocation_x_4 _relativelocation_y_4 _relativelocation_z_4) (`KismetMathLibrary.BreakVector` (`SceneComponent.RelativeLocation` _goaltop)))
  (bind (_boxextent_x _boxextent_y _boxextent_z) (`KismetMathLibrary.BreakVector` (`BoxComponent.BoxExtent` _botbottom)))
  (bind (_boxextent_x_2 _boxextent_y_2 _boxextent_z_2) (`KismetMathLibrary.BreakVector` (`BoxComponent.BoxExtent` _boxtop_2)))
  (bind _returnvalue (`KismetMathLibrary.Conv_IntToDouble` (* (+ _stageparts 1) (/ (`self.StageLength`) 2))))
  (bind _returnvalue_2 (`KismetMathLibrary.Conv_IntToDouble` (- (/ (* (+ (`self.StageParts`) 1) (`self.StageLength`)) 2) (/ (`self.StageLength`) 2))))
  (for _index (range (+ _stageparts 1))
    (bind _returnvalue_3 (`AddComponent|NODE_AddPaperSpriteComponent-0` :`RelativeTransform` (`KismetMathLibrary.MakeTransform` (`KismetMathLibrary.MakeVector` (`KismetMathLibrary.Conv_IntToDouble` (* _index (`self.StageLength`)))))))
    (`PaperSpriteComponent.SetSprite` _returnvalue_3 "/Game/PaperAssets/Background/T_Field_Sprite.T_Field_Sprite"))
  (`BoxComponent.SetBoxExtent` _boxtop_2 (`KismetMathLibrary.MakeVector` _returnvalue _boxextent_y_2 _boxextent_z_2) true)
  (`SceneComponent.K2_SetRelativeLocation` _boxtop (`KismetMathLibrary.MakeVector` _returnvalue_2 _relativelocation_y_2 _relativelocation_z_2) false false)
  (`BoxComponent.SetBoxExtent` _botbottom (`KismetMathLibrary.MakeVector` _returnvalue _boxextent_y _boxextent_z) true)
  (`SceneComponent.K2_SetRelativeLocation` _botbottom_2 (`KismetMathLibrary.MakeVector` _returnvalue_2 _relativelocation_y _relativelocation_z) false false)
  (`SceneComponent.K2_SetRelativeLocation` _goaltop (`KismetMathLibrary.MakeVector` (+ (* (`self.StageParts`) (`self.StageLength`)) _relativelocation_x_4) _relativelocation_y_4 _relativelocation_z_4) false false)
  (`SceneComponent.K2_SetRelativeLocation` _goalbottom (`KismetMathLibrary.MakeVector` (+ (* (`self.StageParts`) (`self.StageLength`)) _relativelocation_x_3) _relativelocation_y_3 _relativelocation_z_3) false false))